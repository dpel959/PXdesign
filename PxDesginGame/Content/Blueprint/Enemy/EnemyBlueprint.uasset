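; Enemy actor that chases the player character once it comes within a fixed range.
; BeginPlay starts an idle animation and caches the player as the target.
; Tick moves it straight toward an in-range player without sweep, turning to face them and starting a looping walk animation on first chase.
; Tick also destroys the enemy when it is flagged dead and plays idle, halting movement, when the player is dead.
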(event `self.ReceiveBeginPlay`
  (`SkeletalMeshComponent.PlayAnimation` (`self.Mesh`) "/Game/Blueprint/Enemy/Enemy_AnimationSeq_Idle.Enemy_AnimationSeq_Idle" true)
  (bind _asfttplayer_character (cast `FTTPlayerCharacter` (`GameplayStatics.GetPlayerCharacter` 0)))
  (set `self.TargetPlayer` _asfttplayer_character))

(event `self.ReceiveTick`
  (params (DeltaSeconds :type "Float (single-precision)"))
  (bind _returnvalue (`self.K2_GetActorLocation`))
  (bind _returnvalue_2 (`self.K2_GetActorLocation` (`self.TargetPlayer`)))
  (if (`self.IsDead`)
    (`self.K2_DestroyActor`)
    (elif (`FTTPlayerCharacter.IsDead` (`self.TargetPlayer`))
      (`SkeletalMeshComponent.PlayAnimation` (`self.Mesh`) "/Game/Blueprint/Enemy/Enemy_AnimationSeq_Idle.Enemy_AnimationSeq_Idle" false)
      (elif (<= (`KismetMathLibrary.Vector_Distance` _returnvalue_2 _returnvalue) 1000.0)
        (if (not (`self.chasing`))
          (`SkeletalMeshComponent.PlayAnimation` (`self.Mesh`) "/Game/Blueprint/Enemy/Enemy_AnimationSeq_Walk1.Enemy_AnimationSeq_Walk1" true)
          (set `self.chasing` true))
        (`self.K2_SetActorLocation` (+ _returnvalue (* (`KismetMathLibrary.Normal` (- _returnvalue_2 _returnvalue)) (* DeltaSeconds (`self.speed`)))))
        (`self.K2_SetActorRotation` (`KismetMathLibrary.FindLookAtRotation` _returnvalue _returnvalue_2))))))

(fn `UserConstructionScript`)