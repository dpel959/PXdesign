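; Destructible wooden crate actor that kills enemies it strikes after being hit by a projectile.
; A hidden static mesh handles movement and hits, while the visible destructible mesh is moved to its location each tick until broken.
; Projectile hits arm the crate, and slowing below a velocity threshold disarms it.
; Hitting an enemy while armed marks it dead and fractures the crate with radius damage, destroying the actor shortly after fracture.
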(event `self.ReceiveTick`
  (params (DeltaSeconds :type "Float (single-precision)"))
  (if (not (`self.IsBroken`))
    (`SceneComponent.K2_SetWorldLocation` (`self.Wooden_Crate_DM`) (`SceneComponent.K2_GetComponentLocation` (`self.StaticMeshComponent`)) true true)
    (if (< (`KismetMathLibrary.VSize` (`SceneComponent.GetComponentVelocity` (`self.StaticMeshComponent`))) 100.0)
      (set `self.HitCount` 0))))

(event `self.ReceiveBeginPlay`
  (`SceneComponent.SetHiddenInGame` (`self.StaticMeshComponent`) true false))

(event `self.StaticMeshComponent.OnComponentHit`
  (params (HitComponent :type "PrimitiveComponent Object Reference") (OtherActor :type "Actor Object Reference") (OtherComp :type "PrimitiveComponent Object Reference") (NormalImpulse :type "Vector Structure") (Hit :type "HitResult Structure (by ref)"))
  (`|ExecutionSequence`
    (:`then_0`
      (cast `ProjectileBase` OtherActor)
      (set `self.HitCount` (+ (`self.HitCount`) 1))
      (`KismetSystemLibrary.PrintString` "Bullet HIt"))
    (:`then_1`
      (if (>= (`self.HitCount`) 1)
        (bind _asenemy_blueprint (cast `/Game/Blueprint/Enemy/EnemyBlueprint` OtherActor))
        (`KismetSystemLibrary.PrintString` "Enemy Hit")
        (set `/Game/Blueprint/Enemy/EnemyBlueprint.IsDead` true _asenemy_blueprint)
        (`DestructibleComponent.ApplyRadiusDamage` (`self.Wooden_Crate_DM`) 10000.0 (`.Location` (`GameplayStatics.BreakHitResult` Hit)) 800.0 10000.0 true)
        (set `self.IsBroken` true)))))

(event `self.Wooden_Crate_DM.OnComponentFracture`
  (params (HitPoint :type "Vector Structure (by ref)") (HitDirection :type "Vector Structure (by ref)"))
  (`KismetSystemLibrary.Delay` 1.0)
  (`self.K2_DestroyActor`))

(fn `UserConstructionScript`)