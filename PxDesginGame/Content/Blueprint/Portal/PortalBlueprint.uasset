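; Portal actor that moves the game to the next level, or triggers the ending when placed in Stage02.
; On any actor overlap it checks the current level name and, outside Stage02, opens the level named by its NextLevel variable.
; In Stage02 it instead loops over every BP_PlayerCharacter, disabling input, showing the mouse cursor and adding an Ending_Blueprint widget to the viewport.
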(event `self.ReceiveActorBeginOverlap`
  (params (OtherActor :type "Actor Object Reference"))
  (bind _returnvalue (`GameplayStatics.GetCurrentLevelName` true))
  (if (`KismetStringLibrary.EqualEqual_StrStr` _returnvalue "Stage02")
    (bind _outactors (`GameplayStatics.GetAllActorsOfClass` "/Game/Blueprint/PlayerCharacter/BP_PlayerCharacter.BP_PlayerCharacter_C"))
    (for _array_element _outactors
      (`self.DisableInput` _array_element null)
      (set `PlayerController.bShowMouseCursor` true (`GameplayStatics.GetPlayerController` 0))
      (bind _returnvalue_2 (`|CreateWidget` "/Game/Blueprint/UI/ending_Blueprint.ending_Blueprint_C"))
      (`UserWidget.AddToViewport` _returnvalue_2 0))
    (else
      (`GameplayStatics.OpenLevel` (`self.NextLevel`)))))

(event `self.ReceiveTick`
  (params (DeltaSeconds :type "Float (single-precision)")))

(fn `UserConstructionScript`)