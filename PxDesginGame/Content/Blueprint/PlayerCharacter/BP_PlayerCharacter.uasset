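; Player character Blueprint with a zoomable camera, a gun with six directional bullet types, and a draining mental power stat.
; Tick lowers MentalPower about once a second through a Delay and feeds it to a dynamic EyeSight material.
; A timeline animates zoom FOV, while next/previous inputs cycle bullet direction.
; Enemy capsule overlap deals damage, disables the player, then shows the death UI after a delay.
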(event `self.ReceiveBeginPlay`
  (`|ExecutionSequence`
    (:`then_0`
      (bind _returnvalue (`|CreateWidget` "/Game/Blueprint/UI/GameUI_Blueprint.GameUI_Blueprint_C"))
      (`UserWidget.AddToViewport` _returnvalue 0))
    (:`then_1`
      (bind _returnvalue_2 (`PrimitiveComponent.CreateDynamicMaterialInstance` (`self.EyeSight`) 0 null "None"))
      (bind _output_get (set `self.DarkSight` _returnvalue_2))
      (`MaterialInstanceDynamic.SetScalarParameterValue` _output_get "EyeSight" 0.3))))

(event `self.ReceiveTick`
  (params (DeltaSeconds :type "Float (single-precision)"))
  (if (not (`self.IsDead`))
    (`|ExecutionSequence`
      (:`then_0`
        (if (> (`self.mentalPower`) 0.0)
          (`MaterialInstanceDynamic.SetScalarParameterValue` (`self.DarkSight`) "EyeSight" (/ (stale _output_get) 100.0))))
      (:`then_1`
        (`KismetSystemLibrary.Delay` 1.0)
        (bind _output_get (set `self.mentalPower` (- (`self.mentalPower`) 0.8)))))))

(event `InputAction|Zoom`
  (params (Key :type "Key Structure"))
  (:`Pressed`
    (set `self.isZoom` true)
    (if (`self.isZoom`) :!label _label
      (bind (_direction _zoom) (`Timeline|Zoom` :!label _label_2)
        (:`Update`
          (`CameraComponent.SetFieldOfView` (`self.Camera`) _zoom)))
      (else
        (goto _label_2 :!via `Reverse`))))
  (:`Released`
    (set `self.isZoom` false)
    (goto _label)))

(event `self.CapsuleComponent.OnComponentBeginOverlap`
  (params (OverlappedComponent :type "PrimitiveComponent Object Reference") (OtherActor :type "Actor Object Reference") (OtherComp :type "PrimitiveComponent Object Reference") (OtherBodyIndex :type Integer) (bFromSweep :type Boolean) (SweepResult :type "HitResult Structure (by ref)"))
  (`KismetSystemLibrary.PrintString` "Overlap")
  (cast `/Game/Blueprint/Enemy/EnemyBlueprint` OtherActor)
  (`self.TakeDamage` 100.0 (`self.DamageEvent`) (`self.GetInstigatorController` OtherActor) OtherActor)
  (`self.SetActorEnableCollision` false)
  (`self.SetActorTickEnabled` false)
  (set `self.bUseControllerRotationYaw` false)
  (`KismetSystemLibrary.Delay` 3.0)
  (bind _returnvalue (`|CreateWidget` "/Game/Blueprint/UI/DeadUI_Blueprint.DeadUI_Blueprint_C"))
  (`UserWidget.AddToViewport` _returnvalue 0)
  (set `PlayerController.bShowMouseCursor` true (`GameplayStatics.GetPlayerController` 0))
  (`self.DisableInput` null)
  (`self.SetActorHiddenInGame` (`self.Gun`) true)
  (`self.SetActorHiddenInGame` true))

(event `InputAction|NextMode`
  (params (Key :type "Key Structure"))
  (:`Pressed`
    (switch `PlayerBulletType` (`self.bulletType`)
      (:`UP`
        (`self.SetBulletTypeDownBP`))
      (:`DOWN`
        (`self.SetBulletTypeRightBP`))
      (:`RIGHT`
        (`self.SetBulletTypeLeftBP`))
      (:`LEFT`
        (`self.SetBulletTypeForwardBP`))
      (:`FORWARD`
        (`self.SetBulletTypeBackwardBP`))
      (:`BACKWARD`
        (`self.SetBulletTypeUPBP`)))))

(event `InputAction|PrevMode`
  (params (Key :type "Key Structure"))
  (:`Pressed`
    (switch `PlayerBulletType` (`self.bulletType`)
      (:`UP`
        (`self.SetBulletTypeBackwardBP`))
      (:`DOWN`
        (`self.SetBulletTypeUPBP`))
      (:`RIGHT`
        (`self.SetBulletTypeDownBP`))
      (:`LEFT`
        (`self.SetBulletTypeRightBP`))
      (:`FORWARD`
        (`self.SetBulletTypeLeftBP`))
      (:`BACKWARD`
        (`self.SetBulletTypeForwardBP`)))))

(fn `UserConstructionScript`)